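; BP_playerController-HUD maps Razer Hydra motion controller input to the player's weapon.
; Movement of controller 1 casts the player character to TheNewGuyController and offsets its WeaponPosition component by scaled controller position.
; That controller's trigger reuses the cast result to call FireMessage on the current weapon.
; Weapon rotation and debug drawing are disconnected, so only position tracks the hand.
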(event `self.HydraControllerMoved`
  (params (Controller :type Integer) (Position :type "Object.Vector Structure") (Velocity :type "Object.Vector Structure") (Acceleration :type "Object.Vector Structure") (Rotation :type "Object.Rotator Structure"))
  (if (== Controller 1)
    (bind _asthenewguycontroller_c (cast `/Game/Blueprints/TheNewGuyController` (`GameplayStatics.GetPlayerCharacter` 0)))
    (`SceneComponent.SetRelativeLocation` (`/Game/Blueprints/TheNewGuyController.weaponPosition` _asthenewguycontroller_c) (+ (50.0 0.0 -20.0) (/ Position 10.0)) false)))

(event `self.HydraTriggerPressed`
  (params (Controller :type Integer))
  ;[1 1 1] Fire
  (if (== Controller 1)
    (message `/Game/Blueprints/playerToWeaponInterface.Fire` (`/Game/Blueprints/TheNewGuyController.CurrentWeapon` (stale `self.HydraControllerMoved` _asthenewguycontroller_c)))))

(fn `UserConstructionScript`)