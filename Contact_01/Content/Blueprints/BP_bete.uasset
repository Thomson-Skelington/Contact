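; BP_bete is a creature that periodically damages the player pawn while TheGuyController overlaps its Colision component.
; Overlap events toggle IsHitting, and a Tick timer applies damage once Cadency has elapsed, printing debug messages.
; A SkeletalMesh2 hit on the bone named "Bone" flags the attack as critical for one Cadency delay, adding CriticalDamages.
; The construction script assigns the M_bete material to the mesh.
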(event `self.colision.OnComponentBeginOverlap`
  (params (OtherActor :type "Actor Object Reference") (OtherComp :type "PrimitiveComponent Object Reference") (OtherBodyIndex :type Integer))
  (cast `/Game/Blueprints/TheGuyController` OtherActor)
  (set `self.isHitting` true))

(event `self.colision.OnComponentEndOverlap`
  (params (OtherActor :type "Actor Object Reference") (OtherComp :type "PrimitiveComponent Object Reference") (OtherBodyIndex :type Integer))
  (cast `/Game/Blueprints/TheGuyController` OtherActor)
  (set `self.isHitting` false))

(event `self.ReceiveTick`
  (params (DeltaSeconds :type "Float (single-precision)"))
  (bind _returnvalue (`GameplayStatics.GetPlayerPawn` 0))
  (bind _timer (`self.Timer`))
  (bind _damages (`self.damages`))
  (set `self.Timer` (+ DeltaSeconds _timer))
  (if (and (>= _timer (`self.cadency`)) (`self.isHitting`))
    (if (`self.isCritical`)
      (`GameplayStatics.ApplyDamage` _returnvalue (+ (`self.criticalDamages`) _damages) null self "/Script/Engine.DamageType")
      (`KismetSystemLibrary.PrintString` "Critical")
      (else
        (`GameplayStatics.ApplyDamage` _returnvalue _damages null self "/Script/Engine.DamageType")))
    (`KismetSystemLibrary.PrintString` "Paf !")
    (set `self.Timer` 0.0)))

(event `self.SkeletalMesh2.OnComponentHit`
  (params (OtherActor :type "Actor Object Reference") (OtherComp :type "PrimitiveComponent Object Reference") (NormalImpulse :type "Object.Vector Structure") (Hit :type "EngineTypes.HitResult Structure (by ref)"))
  (set `self.isCritical` (`KismetStringLibrary.EqualEqual_StrStr` (`KismetStringLibrary.Conv_NameToString` (`.HitBoneName` (`GameplayStatics.BreakHitResult` Hit))) "Bone"))
  (`KismetSystemLibrary.Delay` (`self.cadency`))
  (set `self.isCritical` false))

(fn `UserConstructionScript`
  (`PrimitiveComponent.SetMaterial` (`self.SkeletalMesh2`) 0 "/Game/Meshes/bete/M_bete.M_bete"))