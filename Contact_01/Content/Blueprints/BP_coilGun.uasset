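; Coil gun weapon that builds up to four charges over time and spends them all in a single hitscan shot.
; Tick adds a charge at each ChargeRate interval and lights the matching accumulator meshes.
; Fire line-traces from the Flash component, scaling damage, impulse and sound volume by charge count, then resets the charges.
; The construction script sets the pickup collision, hand positions and unequipped state.
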(event `self.Fire`
  (bind _flash (`self.flash`))
  (bind _flash_2 (`self.flash`))
  (bind _returnvalue (`SceneComponent.K2_GetComponentLocation` _flash))
  (bind _returnvalue_2 (`SceneComponent.GetForwardVector` _flash))
  (bind _returnvalue_3 (`KismetMathLibrary.Conv_IntToDouble` (* (`self.Damage`) (`self.charges`) 1000)))
  ;[1 1 1] Firing
  (`/Engine/EditorBlueprintResources/StandardMacros.CompareInt` (`self.charges`)
    (:`>`
      (`KismetSystemLibrary.PrintString` "Pan !")
      (`GameplayStatics.PlaySoundAtLocation` "/Game/Audio/Template1rst_WeaponFire02.Template1rst_WeaponFire02" (`SceneComponent.K2_GetComponentLocation` _flash_2) (+ (/ (`KismetMathLibrary.Conv_IntToDouble` (`self.charges`)) 8.0) 0.5) 0.8)
      (`ActorComponent.Activate` _flash_2 true)
      ;[1 1 1] InstantHit
      (bind (_outhit _returnvalue_4) (`KismetSystemLibrary.LineTraceSingle` _returnvalue (+ _returnvalue (* _returnvalue_2 (`self.hitDistance`))) "TraceTypeQuery1"))
      (if _returnvalue_4
        (bind (_location _normal _impactpoint _impactnormal _physmat _hitactor _hitcomponent _hitbonename) (`GameplayStatics.BreakHitResult` _outhit))
        (`GameplayStatics.SpawnEmitterAtLocation` "/Game/Particles/P_Explosion.P_Explosion" _impactpoint)
        (`GameplayStatics.ApplyPointDamage` _hitactor _returnvalue_3 _returnvalue_2 _outhit null self)
        (`PrimitiveComponent.AddImpulseAtLocation` _hitcomponent (* _returnvalue_2 _returnvalue_3) _impactpoint _hitbonename)
        (`GameplayStatics.PlaySoundAtLocation` "/Game/Audio/Explosion01.Explosion01" _impactpoint (+ (/ (`KismetMathLibrary.Conv_IntToDouble` (`self.charges`)) 8.0) 0.5) 0.8)
        (`GameplayStatics.ApplyDamage` _hitactor (`KismetMathLibrary.Conv_IntToDouble` (* (`self.Damage`) (`self.charges`))) null self))
      ;[1 1 1] end
      (set `self.charges` 0)
      (set `self.Seconds` 0.0)
      (`PrimitiveComponent.SetMaterial` (`self.charge1`) 0 "/Game/Materials/CoilGun_Accu_OFF.CoilGun_Accu_OFF")
      (`PrimitiveComponent.SetMaterial` (`self.charge2`) 0 "/Game/Materials/CoilGun_Accu_OFF.CoilGun_Accu_OFF")
      (`PrimitiveComponent.SetMaterial` (`self.charge3`) 0 "/Game/Materials/CoilGun_Accu_OFF.CoilGun_Accu_OFF")
      (`PrimitiveComponent.SetMaterial` (`self.charge4`) 0 "/Game/Materials/CoilGun_Accu_OFF.CoilGun_Accu_OFF"))
    (:`==`
      (`KismetSystemLibrary.PrintString` "clic..."))))

(event `self.ReceiveTick`
  (params (DeltaSeconds :type "Float (single-precision)"))
  (bind _seconds (`self.Seconds`))
  (bind _charges (`self.charges`))
  ;[1 1 1] charging
  (set `self.Delta seconds` DeltaSeconds)
  (set `self.Seconds` (+ _seconds (`self.Delta seconds`)))
  (`/Engine/EditorBlueprintResources/StandardMacros.CompareFloat` _seconds (`self.chargeRate`)
    (:`>`
      _)
    (:`==`
      _))
  (set `self.Seconds` 0.0)
  (`/Engine/EditorBlueprintResources/StandardMacros.CompareInt` _charges 4
    (:`<`
      (set `self.charges` (+ _charges 1))
      (`KismetSystemLibrary.PrintString` (`KismetStringLibrary.Conv_IntToString` _charges))
      (switch `int` (`self.charges`)
        (:`1`
          (`PrimitiveComponent.SetMaterial` (`self.charge1`) 0 "/Game/Materials/CoilGun_Accu_ON.CoilGun_Accu_ON"))
        (:`2`
          (`PrimitiveComponent.SetMaterial` (`self.charge1`) 0 "/Game/Materials/CoilGun_Accu_ON.CoilGun_Accu_ON")
          (`PrimitiveComponent.SetMaterial` (`self.charge2`) 0 "/Game/Materials/CoilGun_Accu_ON.CoilGun_Accu_ON"))
        (:`3`
          (`PrimitiveComponent.SetMaterial` (`self.charge1`) 0 "/Game/Materials/CoilGun_Accu_ON.CoilGun_Accu_ON")
          (`PrimitiveComponent.SetMaterial` (`self.charge2`) 0 "/Game/Materials/CoilGun_Accu_ON.CoilGun_Accu_ON")
          (`PrimitiveComponent.SetMaterial` (`self.charge3`) 0 "/Game/Materials/CoilGun_Accu_ON.CoilGun_Accu_ON"))
        (:`4`
          (`PrimitiveComponent.SetMaterial` (`self.charge1`) 0 "/Game/Materials/CoilGun_Accu_ON.CoilGun_Accu_ON")
          (`PrimitiveComponent.SetMaterial` (`self.charge2`) 0 "/Game/Materials/CoilGun_Accu_ON.CoilGun_Accu_ON")
          (`PrimitiveComponent.SetMaterial` (`self.charge3`) 0 "/Game/Materials/CoilGun_Accu_ON.CoilGun_Accu_ON")
          (`PrimitiveComponent.SetMaterial` (`self.charge4`) 0 "/Game/Materials/CoilGun_Accu_ON.CoilGun_Accu_ON"))))))

(fn `UserConstructionScript`
  (set `self.equiped` false)
  (set `self.colliBox` (`self.pickupCollision`))
  ;[1 1 1] hand position
  (set `self.righthandPosition` (`self.righthandPositionSon`))
  (set `self.leftHandPosition` (`self.leftHandPositionSon`)))